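; Enemy actor for a shooter that patrols along X, fires at a random interval and awards score when shot.
; Tick spawns a PusherBP whenever a timer reaches the limit randomized at BeginPlay.
; Tick also reverses movement around a start-relative range, clamping X and adding DeltaTime to direction rather than multiplying, so speed is frame-rate dependent.
; Overlapping a Laser-tagged actor destroys both, spawns an explosion and increments Score_UI directly.
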(event `self.ReceiveBeginPlay`
  (set `self.shootTimerLimit` (`KismetMathLibrary.RandomIntegerInRange` 3 30))
  (set `self.startPos` (`self.K2_GetActorLocation`)))

(event `self.ReceiveActorBeginOverlap`
  (params (OtherActor :type "Actor Object Reference"))
  (if (`ActorComponent.ComponentHasTag` (`Actor.RootComponent` OtherActor) "Laser")
    (`self.K2_DestroyActor` OtherActor)
    (`|SpawnActorFromClass` "/Game/Blueprints/Explosion_BP.Explosion_BP_C" (`KismetMathLibrary.Conv_VectorToTransform` (`SceneComponent.K2_GetComponentLocation` (`self.Cube`))) "Undefined" "OverrideRootScale" null null)
    (bind _foundwidgets (`WidgetBlueprintLibrary.GetAllWidgetsOfClass` "/Game/UI/Score_UI.Score_UI_C"))
    (bind _output (`|GetArrayItem` _foundwidgets))
    (set `/Game/UI/Score_UI.Score` (+ (`/Game/UI/Score_UI.Score` _output) 100) _output)
    (`self.K2_DestroyActor`)))

(event `self.ReceiveTick`
  (params (DeltaSeconds :type "Float (single-precision)"))
  (bind _x (.x (`self.K2_GetActorLocation`)))
  (set `self.deltaTime` DeltaSeconds)
  (bind _output_get (set `self.timer` (+ DeltaSeconds (`self.timer`))))
  (if (>= (`KismetMathLibrary.FTrunc` (`self.timer`)) (`self.shootTimerLimit`))
    (set `self.timer` 0.0)
    (`|SpawnActorFromClass` "/Game/Blueprints/PusherBP.PusherBP_C" (`SceneComponent.K2_GetComponentToWorld` (`self.spawn_location`)) "Undefined" "OverrideRootScale" null null))
  (if (and (> _x (+ (.x (`self.startPos`)) 60.0)) (not (`self.dir`)))
    (set `self.dir` true)
    (set `self.moveDir` -1.0)
    (elif (and (<= _x (.x (`self.startPos`))) (`self.dir`))
      (set `self.dir` false)
      (set `self.moveDir` 1.0)))
  (`self.K2_SetActorLocation` (+ (`KismetMathLibrary.MakeVector` (* (+ (`self.deltaTime`) (`self.moveDir`)) (`self.speed`))) (`KismetMathLibrary.MakeVector` (`KismetMathLibrary.FClamp` _x -200.0 360.0) (.y (`self.K2_GetActorLocation`)) (.z (`self.K2_GetActorLocation`))))))

(fn `UserConstructionScript`)
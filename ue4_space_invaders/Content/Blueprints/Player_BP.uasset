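; Player pawn or actor for a shooter that slides along the X axis and fires lasers.
; BeginPlay enables input and shows the score UI, Horizontal input drives Move within clamped X bounds by a fixed step per call, and Fire spawns LaserBP at SpawnLocation.
; Overlapping a Pusher-tagged actor destroys both, spawns an explosion, sets GameOver, which gates Move and Shoot, and shows ClearStage_UI.
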(event `self.ReceiveActorBeginOverlap`
  (params (OtherActor :type "Actor Object Reference"))
  (if (`ActorComponent.ComponentHasTag` (`Actor.RootComponent` OtherActor) "Pusher")
    (`self.K2_DestroyActor` OtherActor)
    (`|SpawnActorFromClass` "/Game/Blueprints/Explosion_BP.Explosion_BP_C" (`SceneComponent.K2_GetComponentToWorld` (`self.Cube`)) "Undefined" "OverrideRootScale" null null)
    (set `self.GameOver` true)
    (bind _returnvalue (`|CreateWidget` "/Game/UI/ClearStage_UI.ClearStage_UI_C"))
    (`UserWidget.AddToViewport` _returnvalue 0)
    (`self.K2_DestroyActor`)))

(event `self.ReceiveBeginPlay`
  (`self.EnableInput` (`GameplayStatics.GetPlayerController` 0))
  (bind _returnvalue (`|CreateWidget` "/Game/UI/Score_UI.Score_UI_C"))
  (`UserWidget.AddToViewport` _returnvalue 0))

(event `InputAction|Fire`
  (params (Key :type "Key Structure"))
  (:`Pressed`
    (`self.Shoot`)))

(event `InputAxis|Horizontal`
  (params (AxisValue :type "Float (single-precision)"))
  (`self.Move` AxisValue))

(fn `Move`
  (params (`Axis Value` :type "Float (double-precision)"))
  (if (not (`self.GameOver`))
    (`self.K2_SetActorLocation` (+ (`KismetMathLibrary.MakeVector` (* `Axis Value` 5.0)) (`KismetMathLibrary.MakeVector` (`KismetMathLibrary.FClamp` (.x (`self.K2_GetActorLocation`)) -200.0 360.0) (.y (`self.K2_GetActorLocation`)) (.z (`self.K2_GetActorLocation`)))))))

(fn `Shoot`
  (if (not (`self.GameOver`))
    (`|SpawnActorFromClass` "/Game/Blueprints/LaserBP.LaserBP_C" (`SceneComponent.K2_GetComponentToWorld` (`self.spawn_location`)) "Undefined" "OverrideRootScale" null null)))

(fn `UserConstructionScript`)